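; BP_Base_AICharacter is a base NPC character with health, attack, walk speed, patrol and spawn helpers.
; Attack plays a Jump animation directly on the mesh, fires OnAttackEnd immediately, then restores Animation Blueprint mode after a delay.
; ReceiveDamage subtracts from Health without clamping or death handling.
; Helper functions expose health, set walk speed, write the current patrol point to the Blackboard and pick a random spawn transform from a RespawnLocations actor.
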(event Custom|Attack
  (Components|Animation|PlayAnimation (Variables|Character|GetMesh) "/Game/NPC_AI/OLD_NPC/NPC1_William/Jump.Jump" false) ; Do as montage if more complicated animation
  (Default|CallOnAttackEnd) ; Custom event dispatcher
  (Utilities|FlowControl|Delay 2.0) ; Give time to jump
  (Components|Animation|SetAnimationMode (Variables|Character|GetMesh) "AnimationBlueprint" false) ; Reset because Play Animation sets mode to Animation Sequence, so need to set it back to ABP
)

(event Custom|ReceiveDamage
  (params (DamageAmount :type Float%20%28double-precision%29))
  ;[1 1 1] Receive damage and adjust health
  (Variables|Default|SetHealth (- (Variables|Default|GetHealth) DamageAmount)))

(fn ConstructionScript)

(fn GetSpawnTransform
  (bind _returnvalue (Actor|GetActorOfClass "/Game/NPC_AI/RespawnLocations.RespawnLocations_C"))
  (return (Math|Transform|MakeTransform (Utilities|Array|Get(acopy) (Variables|/Game/NPC_AI/RespawnLocations.RespawnLocations_C|GetRespawnLocations _returnvalue) (Math|Random|RandomIntegerinRange 0 (- (Utilities|Array|Length (Variables|/Game/NPC_AI/RespawnLocations.RespawnLocations_C|GetRespawnLocations _returnvalue)) 1))))))

(fn UpdateWalkSpeed
  (params (NewWalkSpeed :type Float%20%28double-precision%29))
  (Variables|/Script/Engine.CharacterMovementComponent|SetMaxWalkSpeed (Variables|Character|GetCharacterMovement) NewWalkSpeed))

(fn GetCurrentHealth
  (return (Variables|Default|GetHealth)))

(fn GetMaxHealth
  (return (Variables|Default|GetMaxHealth)))