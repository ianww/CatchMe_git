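; BP_NPCCharacter7 is a wandering NPC that ragdolls on any damage and respawns elsewhere.
; From BeginPlay it loops AI moves to random reachable points around itself, pausing after each arrival and retrying quickly on failure.
; Damage enables mesh physics and disables capsule collision, then after a delay destroys the actor and spawns a new copy at a random TeleportSystem location.
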(event EventBeginPlay
  (AI|AIMoveTo self (.RandomLocation (AI|Navigation|GetRandomReachablePointinRadius (Transformation|GetActorLocation) 1e+04 0 0)) 0 2e+01 false :!label _label
    (:OnSuccess
      (Utilities|FlowControl|Delay 2.0)
      (goto _label))
    (:OnFail
      (Utilities|FlowControl|Delay 0.2)
      (goto _label))))

(event Collision|EventActorBeginOverlap
  (params (OtherActor :type Actor%20Object%20Reference)))

(event EventTick
  (params (DeltaSeconds :type Float%20%28single-precision%29)))

(event Game|Damage|EventAnyDamage
  (params (Damage :type Float%20%28single-precision%29) (DamageType :type Damage%20Type%20Object%20Reference) (InstigatedBy :type Controller%20Object%20Reference) (DamageCauser :type Actor%20Object%20Reference))
  (Physics|SetSimulatePhysics (Variables|Character|GetMesh) true) ; Will go into ragdoll
  (Collision|SetCollisionEnabled (Variables|Collision|GetCapsuleComponent) "NoCollision") ; Because capsule is still live
  (Utilities|FlowControl|Delay 5.0)
  (Actor|DestroyActor)
  (bind _newparam (CallFunction|GetSpawnTransform))
  (AI|SpawnAIFromClass "BP_NPCCharacter7_C" 0 (.location _newparam) "0, 0, 0" false 0) ; Need to also set AIController Class to Placed in the World or Spawned
)

(fn ConstructionScript)

(fn GetSpawnTransform
  (bind _returnvalue (Actor|GetActorOfClass "/Game/NPC/TeleportSystem.TeleportSystem_C"))
  (return (Math|Transform|MakeTransform (Utilities|Array|Get(acopy) (Variables|/Game/NPC/TeleportSystem.TeleportSystem_C|GetTeleport%20Locations _returnvalue) (Math|Random|RandomIntegerinRange 0 (- (Utilities|Array|Length (Variables|/Game/NPC/TeleportSystem.TeleportSystem_C|GetTeleport%20Locations _returnvalue)) 1))))))