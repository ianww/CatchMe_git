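; BP_NPCCharacter10b is a wandering NPC character that ragdolls and disappears when it takes damage.
; From BeginPlay it loops AI MoveTo toward random reachable points in a large radius around itself, pausing after each arrival and retrying shortly after a failure.
; Any damage turns on mesh physics and disables capsule collision so the body does not block the car, then destroys the actor after a delay.
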(event EventBeginPlay
  (AI|AIMoveTo self (.RandomLocation (AI|Navigation|GetRandomReachablePointinRadius (Transformation|GetActorLocation) 1e+04 0 0)) 0 2e+01 false :!label _label
    (:OnSuccess
      (Utilities|FlowControl|Delay 2.0)
      (goto _label))
    (:OnFail
      (Utilities|FlowControl|Delay 0.2)
      (goto _label))))

(event Collision|EventActorBeginOverlap
  (params (OtherActor :type Actor%20Object%20Reference)))

(event EventTick
  (params (DeltaSeconds :type Float%20%28single-precision%29)))

(event Game|Damage|EventAnyDamage
  (params (Damage :type Float%20%28single-precision%29) (DamageType :type Damage%20Type%20Object%20Reference) (InstigatedBy :type Controller%20Object%20Reference) (DamageCauser :type Actor%20Object%20Reference))
  (Physics|SetSimulatePhysics (Variables|Character|GetMesh) true)
  (Collision|SetCollisionEnabled (Variables|Collision|GetCapsuleComponent) "NoCollision") ; So the car isn't blocked
  (Utilities|FlowControl|Delay 5.0)
  (Actor|DestroyActor))

(fn ConstructionScript)