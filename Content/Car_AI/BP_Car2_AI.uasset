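; BP_Car2_AI is an ambient AI car that drives a looping spline route and deals heavy damage to whatever its mesh hits.
; BeginPlay starts the engine sound and driving animation, then a Timeline moves the skeletal mesh along the spline by distance, restarting after a short delay.
; Logic to stop with a tire screech for the player and later resume is disconnected, so both box overlap events do nothing.
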(event OnComponentBeginOverlap(Box)
  (params (OverlappedComponent :type Primitive%20Component%20Object%20Reference) (OtherActor :type Actor%20Object%20Reference) (OtherComp :type Primitive%20Component%20Object%20Reference) (OtherBodyIndex :type Integer) (bFromSweep :type Boolean) (SweepResult :type Hit%20Result%20Structure%20%28by%20ref%29)))

(event OnComponentEndOverlap(Box)
  (params (OverlappedComponent :type Primitive%20Component%20Object%20Reference) (OtherActor :type Actor%20Object%20Reference) (OtherComp :type Primitive%20Component%20Object%20Reference) (OtherBodyIndex :type Integer)))

(event OnComponentHit(SkeletalMesh)
  (params (HitComponent :type Primitive%20Component%20Object%20Reference) (OtherActor :type Actor%20Object%20Reference) (OtherComp :type Primitive%20Component%20Object%20Reference) (NormalImpulse :type Vector :default "0, 0, 0") (Hit :type Hit%20Result%20Structure%20%28by%20ref%29))
  (Game|Damage|ApplyDamage OtherActor 1e+03 0 0))

(event Custom|StopCar
  (bind _carspeed (Timeline|Timeline Stop)
    (:Update
      (Transformation|SetWorldLocationAndRotation (Variables|Default|GetSkeletalMesh) (.location (Spline|GetTransformatDistanceAlongSpline (Variables|Default|GetSpline) (Math|Float|Lerp 0.0 (Spline|GetSplineLength (Variables|Default|GetSpline)) _carspeed) "World" false)) (.rotation (Spline|GetTransformatDistanceAlongSpline (Variables|Default|GetSpline) (Math|Float|Lerp 0.0 (Spline|GetSplineLength (Variables|Default|GetSpline)) _carspeed) "World" false)) false false))
    (:Finished
      (Utilities|FlowControl|Delay 0.1)
      (Timeline|Timeline PlayFromStart))))

(event Custom|PlayCar
  (bind _carspeed (Timeline|Timeline Play)
    (:Update
      (Transformation|SetWorldLocationAndRotation (Variables|Default|GetSkeletalMesh) (.location (Spline|GetTransformatDistanceAlongSpline (Variables|Default|GetSpline) (Math|Float|Lerp 0.0 (Spline|GetSplineLength (Variables|Default|GetSpline)) _carspeed) "World" false)) (.rotation (Spline|GetTransformatDistanceAlongSpline (Variables|Default|GetSpline) (Math|Float|Lerp 0.0 (Spline|GetSplineLength (Variables|Default|GetSpline)) _carspeed) "World" false)) false false))
    (:Finished
      (Utilities|FlowControl|Delay 0.1)
      (Timeline|Timeline PlayFromStart))))

(event EventBeginPlay
  (bind _audio (Variables|Default|GetAudio))
  (Audio|Components|Audio|SetSound _audio "/Game/Car_AI/carEngine.carEngine")
  (Audio|Components|Audio|Play _audio 0.0)
  (Components|Animation|PlayAnimation (Variables|Default|GetSkeletalMesh) "/Game/Car_AI/SK_Car2Moving.SK_Car2Moving" true)
  (bind _carspeed (Timeline|Timeline PlayFromStart)
    (:Update
      (Transformation|SetWorldLocationAndRotation (Variables|Default|GetSkeletalMesh) (.location (Spline|GetTransformatDistanceAlongSpline (Variables|Default|GetSpline) (Math|Float|Lerp 0.0 (Spline|GetSplineLength (Variables|Default|GetSpline)) _carspeed) "World" false)) (.rotation (Spline|GetTransformatDistanceAlongSpline (Variables|Default|GetSpline) (Math|Float|Lerp 0.0 (Spline|GetSplineLength (Variables|Default|GetSpline)) _carspeed) "World" false)) false false))
    (:Finished
      (Utilities|FlowControl|Delay 0.1)
      (Timeline|Timeline PlayFromStart))))

(fn ConstructionScript)